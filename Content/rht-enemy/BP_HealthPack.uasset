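; BP_HealthPack is a health pickup that heals the player on contact and can be destroyed by bullets.
; A Box overlap with BP_Character calls HealMe and removes the pack, while an overlap with BP_Bullet destroys both pack and bullet without healing.
; HealMe adds a fixed amount to Health in the Gameinstance_zzk cached at BeginPlay, capped at MaxHealth.
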(event `self.ReceiveBeginPlay`
  (bind _asbp_character (cast `/Game/InfimaGames/FreeFPSTemplate/Core/BP_Character` (`GameplayStatics.GetPlayerCharacter` 0)))
  (set `self.主角` _asbp_character)
  (bind _asgameinstance_zzk (cast `/Game/zzk——UI/Gameinstance_zzk` (`GameplayStatics.GetGameInstance`)))
  (set `self.data` _asgameinstance_zzk))

(event `self.Box.OnComponentBeginOverlap`
  (params (OverlappedComponent :type "PrimitiveComponent Object Reference") (OtherActor :type "Actor Object Reference") (OtherComp :type "PrimitiveComponent Object Reference") (OtherBodyIndex :type Integer) (bFromSweep :type Boolean) (SweepResult :type "HitResult Structure (by ref)"))
  (cast `/Game/InfimaGames/FreeFPSTemplate/Core/BP_Character` OtherActor
    (:`then`
      (`self.Heal Me!`)
      (`self.K2_DestroyActor`))
    (:`CastFailed`
      (bind _asbp_bullet (cast `/Game/InfimaGames/FreeFPSTemplate/Core/BP_Bullet` OtherActor))
      (`self.K2_DestroyActor`)
      (`self.K2_DestroyActor` _asbp_bullet))))

(event `self.HealthPack.OnComponentHit`
  (params (HitComponent :type "PrimitiveComponent Object Reference") (OtherActor :type "Actor Object Reference") (OtherComp :type "PrimitiveComponent Object Reference") (NormalImpulse :type "Vector Structure") (Hit :type "HitResult Structure (by ref)")))

(event `self.ReceiveTick`
  (params (DeltaSeconds :type "Float (single-precision)")))

(fn `Heal Me!`
  (bind _data (`self.data`))
  (bind _returnvalue (+ 5.0 (`/Game/zzk——UI/Gameinstance_zzk.health` (`self.data`))))
  (if (<= (`/Game/zzk——UI/Gameinstance_zzk.Max Health` (`self.data`)) _returnvalue)
    (set `/Game/zzk——UI/Gameinstance_zzk.health` (`/Game/zzk——UI/Gameinstance_zzk.Max Health` _data) _data)
    (else
      (set `/Game/zzk——UI/Gameinstance_zzk.health` _returnvalue (`self.data`)))))

(fn `UserConstructionScript`)